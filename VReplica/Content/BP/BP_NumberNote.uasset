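; BP_NumberNote is an actor that displays a number as rendered text and randomly shifts its position at game start.
; The construction script writes the Number variable into the TextRender component.
; On BeginPlay, only the authority offsets the root component without sweeping, by a random vector scaled by MaxRandomDistance.
; Each random component spans 0 to 1 before scaling, so the shift is not centered on the original position.
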(event EventBeginPlay
  (Networking|SwitchHasAuthority
    (:Authority
      (Variables|Default|SetRandomVector (Math|Vector|MakeVector (Math|Random|RandomFloat) (Math|Random|RandomFloat) (Math|Random|RandomFloat)))
      (Transformation|AddWorldOffset (Variables|Default|GetDefaultSceneRoot) (* (Variables|Default|GetRandomVector) (Variables|Default|GetMaxRandomDistance)) false false))))

(event Collision|EventActorBeginOverlap
  (params (OtherActor :type Actor%20Object%20Reference)))

(event EventTick
  (params (DeltaSeconds :type Float%20%28single-precision%29)))

(fn ConstructionScript
  (Rendering|Components|TextRender|SetText (Variables|Default|GetTextRender) (Utilities|Text|ToText(Integer) (Variables|Default|GetNumber))))