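; VR pawn that spawns left and right hand actors on a floor-level tracking origin and attaches them to its VR origin.
; A VRCalibrate input moves its root, and that of a MotionControllerPawn in the level, to the PlayerStart.
; It then repositions both VR origins using this pawn's camera offset and inverted yaw, cancelling horizontal headset offset while keeping PlayerStart height.
; An event toggles avatar mesh visibility.
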(event EventBeginPlay
  (bind _returnvalue (Math|Transform|MakeTransform "0, 0, 0"))
  (bind _self self)
  (bind _vrorigin (Variables|Default|GetVROrigin))
  (Utilities|FlowControl|Sequence
    (:then_0
      (Class|HeadMountedDisplayFunctionLibrary|SetTrackingOrigin "Floor"))
    (:then_1
      (Utilities|FlowControl|Sequence
        (:then_0
          (bind _returnvalue_2 (Game|SpawnActorfromClass "/Game/BP_Hand.BP_Hand_C" _returnvalue "Undefined" _self "Left" 0))
          (bind _output_get (Variables|Default|SetLeftHand _returnvalue_2))
          (Transformation|AttachComponentToComponent _output_get _vrorigin "None" "KeepRelative" "KeepRelative" "KeepRelative" true))
        (:then_1
          (bind _returnvalue_3 (Game|SpawnActorfromClass "/Game/BP_RightHand.BP_RightHand_C" _returnvalue "Undefined" _self "Right" 0))
          (bind _output_get_2 (Variables|Default|SetRightHand _returnvalue_3))
          (Transformation|AttachComponentToComponent _output_get_2 _vrorigin "None" "KeepRelative" "KeepRelative" "KeepRelative" true))))))

(event Collision|EventActorBeginOverlap
  (params (OtherActor :type Actor%20Object%20Reference)))

(event EventTick
  (params (DeltaSeconds :type Float%20%28single-precision%29)))

(event EventSetAvatarVisibility
  (params (Visibility :type Boolean))
  (Rendering|SetVisibility (Variables|Default|GetStaticMesh) Visibility false))

(event Input|ActionEvents|InputActionVRCalibrate
  (params (Key :type Key%20Structure :default "None"))
  (bind _camera (Variables|Default|GetCamera))
  (bind _returnvalue (Transformation|GetRelativeTransform _camera))
  (bind _returnvalue_2 (Class|KismetMathLibrary|NegateRotator (.rotation _returnvalue)))
  (bind _returnvalue_3 (Math|Rotator|MakeRotator 0.0 0.0 (.yaw _returnvalue_2)))
  (:Pressed
    (bind _returnvalue_4 (Actor|GetActorOfClass "/Script/Engine.PlayerStart"))
    (bind _returnvalue_5 (Actor|GetActorOfClass "/Game/VirtualRealityBP/Blueprints/MotionControllerPawn.MotionControllerPawn_C"))
    (Transformation|SetWorldLocationAndRotation (Variables|Default|GetDefaultSceneRoot) (Transformation|GetActorLocation _returnvalue_4) (Transformation|GetActorRotation _returnvalue_4) false false)
    (Transformation|SetWorldLocationAndRotation (Variables|Default|GetVROrigin) (Math|Vector|MakeVector (.x (- (Transformation|GetActorLocation _returnvalue_4) (Math|Vector|RotateVector (.location _returnvalue) _returnvalue_3))) (.y (- (Transformation|GetActorLocation _returnvalue_4) (Math|Vector|RotateVector (.location _returnvalue) _returnvalue_3))) (.Z (Math|Vector|BreakVector (Transformation|GetActorLocation _returnvalue_4)))) _returnvalue_3 false false)))

(fn ConstructionScript)